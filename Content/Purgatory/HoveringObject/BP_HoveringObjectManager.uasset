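; Manager actor that drifts and tumbles randomly chosen meshes past its location in a repeating cycle.
; On BeginPlay it spawns one BP_HoveringObject per listed mesh as a reusable pool at a reset location.
; Each cycle scatters up to Amount random pool members around the manager, then a Hover timeline moves them along world X while rotating them.
; When the timeline finishes, they return to the reset location and a new selection starts.
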(event Custom|StartHover
  (bind _alpha (Timeline|Hover Play)
    (:Update
      (bind _output_get (Variables|Default|SetAlpha _alpha))
      (for _array_element (Variables|Default|GetCurrentObjects)
        (Transformation|AddActorWorldOffset _array_element (Math|Vector|MakeVector (* _output_get (* -1.0 (Variables|Default|GetSpeedMultiplier))) 0.0 0.0))
        (Transformation|AddActorLocalRotation _array_element (Math|Rotator|MakeRotator (Variables|Default|GetAlpha) (Variables|Default|GetAlpha) (Variables|Default|GetAlpha)) false false)))
    (:Finished
      (CallFunction|ResetCurrentObjects)
      (CallFunction|SetCurrentObjects)
      (CallFunction|SetTime)
      (CallFunction|StartHover))))

(event Custom|SetTime
  (bind _alpha (Timeline|Hover SetNewTime)
    (:Update
      (bind _output_get (Variables|Default|SetAlpha _alpha))
      (for _array_element (Variables|Default|GetCurrentObjects)
        (Transformation|AddActorWorldOffset _array_element (Math|Vector|MakeVector (* _output_get (* -1.0 (Variables|Default|GetSpeedMultiplier))) 0.0 0.0))
        (Transformation|AddActorLocalRotation _array_element (Math|Rotator|MakeRotator (Variables|Default|GetAlpha) (Variables|Default|GetAlpha) (Variables|Default|GetAlpha)) false false)))
    (:Finished
      (CallFunction|ResetCurrentObjects)
      (CallFunction|SetCurrentObjects)
      (CallFunction|SetTime)
      (CallFunction|StartHover))))

(event EventBeginPlay
  (if (> (Variables|Default|GetAmount) 0)
    (CallFunction|SpawnObjects)
    (CallFunction|SetCurrentObjects)
    (CallFunction|SetTime)
    (CallFunction|StartHover)))

(fn ConstructionScript)

(fn SetCurrentObjects
  (bind _objectoffsetmin (Variables|Default|GetObjectOffsetMin))
  (bind _objectoffsetmax (Variables|Default|GetObjectOffsetMax))
  (bind _spawnedobjects (Variables|Default|GetSpawnedObjects))
  (bind _spawnedobjects_2 (Variables|Default|GetSpawnedObjects))
  (bind _returnvalue (Utilities|Array|Length _spawnedobjects))
  (bind _returnvalue_2 (Math|Random|RandomFloatinRange _objectoffsetmin _objectoffsetmax))
  (bind _returnvalue_3 (- _returnvalue 1))
  (bind _returnvalue_4 (Math|Random|RandomInteger _returnvalue_3))
  (bind _output (Utilities|Array|Get(acopy) _spawnedobjects_2 _returnvalue_4))
  (Utilities|Array|Clear (Variables|Default|GetCurrentObjects))
  (for _index (range 0 (- (Variables|Default|GetAmount) 1))
    (Utilities|IsValid _output
      (:Is%20Valid
        (Utilities|Array|AddUnique (Variables|Default|GetCurrentObjects) _output))))
  (for _array_element (Variables|Default|GetCurrentObjects)
    (Transformation|SetActorLocation _array_element (+ (Transformation|GetActorLocation) (Math|Vector|MakeVector _returnvalue_2 _returnvalue_2 _returnvalue_2)) false false)))

(fn ResetCurrentObjects
  (for _array_element (Variables|Default|GetCurrentObjects)
    (Transformation|SetActorLocation _array_element (Variables|Default|GetResetLocation) false false)))

(fn SpawnObjects
  (for _array_element (Variables|Default|GetObjects)
    (bind _returnvalue (Game|SpawnActorfromClass "/Game/Purgatory/HoveringObject/BP_HoveringObject.BP_HoveringObject_C" (Math|Conversions|ToTransform(Vector) (Variables|Default|GetResetLocation)) "Undefined" 0 0))
    (Components|StaticMesh|SetStaticMesh (Variables|/Game/Purgatory/HoveringObject/BP_HoveringObject.BP_HoveringObject_C|GetStaticMesh _returnvalue) _array_element)
    (Rendering|Material|SetMaterial (Variables|/Game/Purgatory/HoveringObject/BP_HoveringObject.BP_HoveringObject_C|GetStaticMesh _returnvalue) 0 (Rendering|Material|GetMaterial _array_element 0))
    (Utilities|Array|AddUnique (Variables|Default|GetSpawnedObjects) _returnvalue)))