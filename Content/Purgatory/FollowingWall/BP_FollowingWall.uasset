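; BP_FollowingWall is a Purgatory wall actor that, judging by its name and timer-driven movement, follows the player.
; On BeginPlay, after a short delay, it copies four mesh distance values, caches the player character and starting facing, calculates its location and starts a movement timer.
; SetStart records position and yaw, which Restart uses to reset the wall.
; The movement and location logic is defined outside these graphs.
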(event EventBeginPlay
  (Utilities|FlowControl|Delay 0.1)
  (Variables|Default|SetDistanceFirst (Variables|Default|GetDistanceMeshFirst))
  (Variables|Default|SetDistanceSecond (Variables|Default|GetDistanceMeshSecond))
  (Variables|Default|SetDistanceThird (Variables|Default|GetDistanceMeshThird))
  (Variables|Default|SetDistanceFourth (Variables|Default|GetDistanceMeshFourth))
  (Variables|Default|SetPlayerCharacter (Game|GetPlayerCharacter 0))
  (Variables|Default|SetPlayerFacingStart (Transformation|GetActorForwardVector (Variables|Default|GetPlayerCharacter)))
  (Class|FollowingWall|CalculateLocation)
  (Class|FollowingWall|StartMoveActorTimer))

(event EventSetStart
  (Variables|Default|SetStartPosition (Transformation|GetActorLocation))
  (Variables|Default|SetStartRotation (.Yaw (Math|Rotator|BreakRotator (Transformation|GetActorRotation)))))

(event EventRestart
  (Class|FollowingWall|ResetWall (Variables|Default|GetStartPosition))
  (Class|FollowingWall|SetYawRotation (Variables|Default|GetStartRotation)))

(fn ConstructionScript)