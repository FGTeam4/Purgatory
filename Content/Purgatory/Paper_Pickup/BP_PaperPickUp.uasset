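; Numbered collectible paper page that hovers and spins, then on pickup hides, plays a sound and points the way to the next page.
; The trail lerps a straight line to NextPickup into a spline, spawns meshes along it through a delayed-loop macro, then clears them after a delay.
; A looping timer toggles custom-depth outlining by player distance.
; Ending pages register with the Lars character, and Restart restores position and visibility.
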(event Custom|Pick
  (Development|SetHiddeninGame (Variables|Default|GetPageMesh) true true)
  (Collision|SetCollisionEnabled (Variables|Default|GetSphere) "NoCollision")
  (CallFunction|ShowPath)
  (Audio|PlaySoundatLocation "/Game/Purgatory/Sounds/SFX/SoundFiles/Picking_upp_paper.Picking_upp_paper" (Transformation|GetActorLocation) "0, 0, 0" 1.0 1.0 0.0 0 0 0)
  (if (Variables|Default|GetbIsEndingPage)
    (Variables|/Game/Purgatory/Character/Lars/BP_Character_Lars.BP_Character_Lars_C|SetCurrentReadPage (Variables|Default|GetCharacter) self)))

(event Custom|Reset
  (Development|SetHiddeninGame (Variables|Default|GetPageMesh) false true)
  (Development|SetHiddeninGame (Variables|Default|GetSphere) true false)
  (Collision|SetCollisionEnabled (Variables|Default|GetSphere) "QueryOnly"))

(event Custom|ShowPath
  (Utilities|IsValid (Variables|Trail|GetNextPickup)
    (:Is%20Valid
      (bind _path (Trail|FindPath))
      (Trail|BuildSpline _path)
      (Utilities|BuildPath
        (:out
          (Utilities|FlowControl|Delay (Variables|Trail|GetTimeBeforeClearPath))
          (Trail|ClearSpline))))))

(event Custom|CheckDistanceMaterial
  (Rendering|SetRenderCustomDepth (Variables|Default|GetPageMesh) (<= (Math|Vector|Distance(Vector) (Transformation|GetActorLocation) (Transformation|GetActorLocation (Variables|Default|GetCharacter))) (Variables|Default|GetOutlineDistance))))

(event EventBeginPlay
  (CallFunction|SetStart)
  (bind _asbp_character_lars (Utilities|Casting|CastToBP_Character_Lars (Game|GetPlayerCharacter 0)))
  (Variables|Default|SetCharacter _asbp_character_lars)
  (Transformation|AddLocalRotation (Variables|Default|GetPageMesh) (Math|Rotator|MakeRotator 0.0 0.0 (Math|Random|RandomFloatinRange 0.0 3.6e+02)) false false)
  (Variables|Animation|SetRandomHeightOffset (Math|Random|RandomFloatinRange 0.0 5.0))
  (Utilities|Time|SetTimerbyEvent (delegate Custom|CheckDistanceMaterial) 0.5 true))

(event EventSetStart
  (Variables|Restart|SetStartPosition (Transformation|GetActorLocation)))

(event EventTick
  (params (DeltaSeconds :type Float%20%28single-precision%29))
  (CallFunction|Animation DeltaSeconds))

(event EventRestart
  (Transformation|SetActorLocation (Variables|Restart|GetStartPosition) false false)
  (CallFunction|Reset))

(fn ConstructionScript
  (bind _numberinsequence (Variables|Default|GetNumberInSequence))
  (bind _returnvalue (+ _numberinsequence 1))
  (bind _returnvalue_2 (Utilities|Text|ToText(Integer) _returnvalue))
  (Rendering|Components|TextRender|SetText (Variables|Default|GetFrontText) _returnvalue_2)
  (Rendering|Components|TextRender|SetText (Variables|Default|GetBackText) _returnvalue_2)
  (if (== _returnvalue 1)
    (Transformation|SetRelativeLocation (Variables|Default|GetFrontText) "1.800000,0.369256,10.000000" false false)
    (Transformation|SetRelativeLocation (Variables|Default|GetBackText) "-1.500000,1.236539,10.383277" false false)))

(fn Animation
  (params (Delta :type Float%20%28single-precision%29))
  (Transformation|AddLocalOffset (Variables|Default|GetPageMesh) (Math|Vector|MakeVector 0.0 0.0 (* (Math|Trig|Cos(Radians) (* (+ (Actor|GetGameTimeSinceCreation) (Variables|Animation|GetRandomHeightOffset)) (Variables|Animation|GetSpeedMultiplier))) (Variables|Animation|GetHeightMultiplier))) false false)
  (Transformation|AddLocalRotation (Variables|Default|GetPageMesh) (Math|Rotator|MakeRotator 0.0 0.0 (* (Variables|Animation|GetRotationSpeed) (Math|Random|RandomFloatinRange 0.7 1.3))) false false))

(fn BuildSpline
  (params (Path :type Array%20of%20Vectors))
  (for _array_element Path
    (Spline|AddSplinePoint (Variables|Default|GetSpline) _array_element "World" true)))

(fn ClearSpline
  (Spline|ClearSplinePoints (Variables|Default|GetSpline) true)
  (for _array_element (Variables|Trail|GetTrailWaypoints)
    (Components|DestroyComponent _array_element))
  (Utilities|Array|Clear (Variables|Trail|GetTrailWaypoints)))

(fn FindPath
  (for _index (range 0 (Variables|Trail|GetSplineQuality))
    (Utilities|Array|Add (LocalVariables|GetpathPoints) (Math|Vector|Lerp(Vector) (Transformation|GetActorLocation) (Transformation|GetActorLocation (Variables|Trail|GetNextPickup)) (/ (Math|Conversions|ToFloat(Integer) _index) (Math|Conversions|ToFloat(Integer) (Variables|Trail|GetSplineQuality))))))
  (return (LocalVariables|GetpathPoints)))