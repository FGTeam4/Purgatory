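; Checkpoint actor that updates the Lars character's current checkpoint when he enters its trigger.
; On overlap, it stores itself on the character and calls SetStart, skipping checkpoints that are already current.
; BeginPlay prints red setup warnings for an unset EndPortal and for the room's Papers list, though the Papers check appears inverted, warning when the list is non-empty.
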(event OnComponentBeginOverlap(Trigger)
  (params (OverlappedComponent :type Primitive%20Component%20Object%20Reference) (OtherActor :type Actor%20Object%20Reference) (OtherComp :type Primitive%20Component%20Object%20Reference) (OtherBodyIndex :type Integer) (bFromSweep :type Boolean) (SweepResult :type Hit%20Result%20Structure%20%28by%20ref%29))
  (bind _asbp_character_lars (Utilities|Casting|CastToBP_Character_Lars OtherActor))
  (if (not (== (Variables|/Game/Purgatory/Character/Lars/BP_Character_Lars.BP_Character_Lars_C|GetCurrentCheckpoint _asbp_character_lars) self))
    (Variables|/Game/Purgatory/Character/Lars/BP_Character_Lars.BP_Character_Lars_C|SetCurrentCheckpoint _asbp_character_lars self)
    (Default|SetStart _asbp_character_lars)))

(event EventBeginPlay
  (if (== (Utilities|Array|Length (Variables|Pickups|GetPapers)) 0)
    _
    (else
      (Development|PrintString "You need to set which papers affect this room!" true true "(R=1.000000,G=0.000000,B=0.049778,A=1.000000)")))
  (if (not (Utilities|IsValid (Variables|Pickups|GetEndPortal)))
    (Development|PrintString "You need to set your end portal!" true true "(R=1.000000,G=0.000000,B=0.061032,A=1.000000)")))

(event Collision|EventActorBeginOverlap
  (params (OtherActor :type Actor%20Object%20Reference)))

(event EventTick
  (params (DeltaSeconds :type Float%20%28single-precision%29)))

(fn ConstructionScript)