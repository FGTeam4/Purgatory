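; Player character Lars for Purgatory, handling paper collection, a readable notebook, pushing audio, idle detection, pause and game UI.
; Papers picked up in sequence open the checkpoint's portal; closing the notebook with an ending page collected plays the ending cinematic.
; Holding R ramps screen blur through looping timers, then restarts all IRestart actors.
; Teleporting resets papers from a non-looping one onward, and debug keys jump between checkpoints via level streaming.
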(event OnComponentBeginOverlap(CapsuleComponent)
  (params (OverlappedComponent :type Primitive%20Component%20Object%20Reference) (OtherActor :type Actor%20Object%20Reference) (OtherComp :type Primitive%20Component%20Object%20Reference) (OtherBodyIndex :type Integer) (bFromSweep :type Boolean) (SweepResult :type Hit%20Result%20Structure%20%28by%20ref%29))
  ;[1 0.9265 0.2541] Collision
  ;;[1 1 1] if correct paper, add to list and hide
  (bind _asbp_paper_pick_up (Utilities|Casting|CastToBP_PaperPickUp OtherActor))
  (if (== (Variables|/Game/Purgatory/Paper_Pickup/BP_PaperPickUp.BP_PaperPickUp_C|GetNumberInSequence _asbp_paper_pick_up) (Utilities|Array|Length (Variables|Papers|GetPapers)))
    (Variables|Papers|SetCurrentPaper _asbp_paper_pick_up)
    (Default|Pick (Variables|Papers|GetCurrentPaper))
    (Utilities|Array|Add (Variables|Papers|GetPapers) (Variables|Papers|GetCurrentPaper))
    (Variables|Checks|SetbPickingUp true)
    ;;[1 1 1] Add Readable Pages
    (bind _returnvalue (Utilities|Array|AddUnique (Variables|UI|GetReadablePages) (Variables|Papers|GetCurrentPaper)))
    (Variables|UI|SetpageIndex _returnvalue)
    (Variables|UI|SetCurrentReadPage (Variables|Papers|GetCurrentPaper))
    ;;[1 1 1] Activates Read Paper in UI
    (Variables|Papers|SetbHasPapers true)
    (if (and (== (Utilities|Array|Length (Variables|Papers|GetPapers)) 1) (not (Variables|UI|GetbPaperIsVisible)))
      (Default|SetReadPageVisibility (Variables|UI|GetGameUI) "Visible")
      (Utilities|Time|SetTimerbyEvent (delegate Custom|ClearReadPage) 4.0))
    ;;[1 1 1] Opens Portal when collected all papers
    (if (== (Utilities|Array|Length (Variables|Papers|GetPapers)) (Utilities|Array|Length (Variables|/Game/Purgatory/Checkpoint/BP_Checkpoint.BP_Checkpoint_C|GetPapers (Variables|Checkpoints|GetCurrentCheckpoint))))
      (Default|Deactivate (Variables|/Game/Purgatory/Checkpoint/BP_Checkpoint.BP_Checkpoint_C|GetEndPortal (Variables|Checkpoints|GetCurrentCheckpoint)))
      (Audio|Components|Audio|Play (Variables|Default|GetLevelComplete) 0.0))))

(event OnComponentBeginOverlap(PushableCollision)
  (params (OverlappedComponent :type Primitive%20Component%20Object%20Reference) (OtherActor :type Actor%20Object%20Reference) (OtherComp :type Primitive%20Component%20Object%20Reference) (OtherBodyIndex :type Integer) (bFromSweep :type Boolean) (SweepResult :type Hit%20Result%20Structure%20%28by%20ref%29))
  ;[1 0.9265 0.2541] Collision
  ;;[1 1 1] Temprorary solution to chedk whether touching a pushbox
  (Utilities|Casting|CastToBP_PushableObject OtherActor
    (:then
      _)
    (:CastFailed
      (Utilities|Casting|CastToBP_PushBox OtherActor)))
  (Variables|Checks|SetbTouchingPushable true)
  (if (not (Audio|Components|Audio|IsPlaying (Variables|Components|GetPushingBoxAudio)))
    (Audio|Components|Audio|Play (Variables|Components|GetPushingBoxAudio) 0.0)))

(event OnComponentEndOverlap(PushableCollision)
  (params (OverlappedComponent :type Primitive%20Component%20Object%20Reference) (OtherActor :type Actor%20Object%20Reference) (OtherComp :type Primitive%20Component%20Object%20Reference) (OtherBodyIndex :type Integer))
  ;[1 0.9265 0.2541] Collision
  ;;[1 1 1] Temprorary solution to chedk whether touching a pushbox
  (Utilities|Casting|CastToBP_PushableObject OtherActor
    (:then
      _)
    (:CastFailed
      (Utilities|Casting|CastToBP_PushBox OtherActor)))
  (Variables|Checks|SetbTouchingPushable false)
  (if (Audio|Components|Audio|IsPlaying (Variables|Components|GetPushingBoxAudio))
    (Audio|Components|Audio|Stop (Variables|Components|GetPushingBoxAudio))))

(event Custom|Teleport
  ;[1 1 1] OnTeleport
  (Utilities|ResetNonTeleportablePapers
    (:Completed
      (Default|CallOnTeleport))))

(event Custom|TurnPage
  (params (TurnPage :type ETurnPage%20Enum :default "NewEnumerator0"))
  (bind _readablepages (Variables|UI|GetReadablePages))
  (bind _returnvalue (Utilities|Array|Length _readablepages))
  ;[0.7653 1 0.6506] UI
  (if (Utilities|Enum|Equal(Enum) TurnPage "NewEnumerator0")
    (bind _result (Math|Integer|DecrementInt (Variables|UI|GetpageIndex))
      (:%20%20
        (if (< _result 0)
          (Variables|UI|SetpageIndex 0)
          (else
            (CallFunction|SetCurrentPageVisibility "Hidden" :!label _label)
            (Variables|UI|SetCurrentReadPage (Utilities|Array|Get(acopy) (Variables|UI|GetReadablePages) (Variables|UI|GetpageIndex)))
            (CallFunction|SetCurrentPageVisibility "Visible")
            (Audio|PlaySoundatLocation "/Game/Purgatory/Sounds/SFX/SoundFiles/Open_notebook.Open_notebook" (Transformation|GetActorLocation) "0, 0, 0" 1.0 1.0 0.0 0 0 0)
            (if (Utilities|Enum|Equal(Enum) TurnPage "NewEnumerator0")
              (Variables|Checks|SetbFlipLeft true)
              (else
                (Variables|Checks|SetbFlipRight true)))))))
    (else
      (bind _result_2 (Math|Integer|IncrementInt (Variables|UI|GetpageIndex))
        (:%20%20
          (if (>= _result_2 _returnvalue)
            (Variables|UI|SetpageIndex (- _returnvalue 1))
            (else
              (goto _label))))))))

(event Custom|PlayEndingCinematic
  (bind _endcinematicplayer (Variables|Default|GetEndCinematicPlayer))
  ;[1 1 1] Ending Cinematic
  (bind _returnvalue (UserInterface|CreateWidget "/Game/Purgatory/Cinematics/WBP_EndCinematic.WBP_EndCinematic_C" (Game|GetPlayerController 0)))
  (UserInterface|Viewport|AddtoViewport _returnvalue 0)
  (Media|MediaPlayer|OpenSource _endcinematicplayer "/Game/Purgatory/Cinematics/EndSequence.EndSequence")
  (EventDispatchers|AssignOnEndReached _endcinematicplayer (delegate Custom|OnEndReached_Event_0)))

(event Custom|OnEndReached_Event_0
  ;[1 1 1] Ending Cinematic
  (Utilities|FlowControl|Delay (Variables|Default|GetEndingCinematicDelay))
  (Widget|RemovefromParent (stale Custom|PlayEndingCinematic _returnvalue))
  (bind _asgi_purgatory (Utilities|Casting|CastToGI_Purgatory (Game|GetGameInstance)))
  (Variables|/Game/Purgatory/Globals/GameInstance/GI_Purgatory.GI_Purgatory_C|SetGameWon _asgi_purgatory true)
  (Game|OpenLevel(byName) "MainMenu"))

(event Custom|OpenBook
  ;[0.7653 1 0.6506] UI
  (Utilities|IsValid (Variables|UI|GetCurrentReadPage)
    (:Is%20Valid
      (Default|SetReadPageVisibility (Variables|UI|GetGameUI) "Hidden")
      (Variables|UI|SetbPaperIsVisible true))))

(event Custom|CloseBook
  ;[0.7653 1 0.6506] UI
  (Utilities|IsValid (Variables|UI|GetCurrentReadPage)
    (:Is%20Valid
      (CallFunction|SetCurrentPageVisibility "Hidden")
      (Default|SetClosePageVisibility (Variables|UI|GetGameUI) "Hidden")
      (Variables|UI|SetbPaperIsVisible false)
      (Variables|UI|SetbCanTurnPage false)
      (for _array_element (Variables|Papers|GetPapers)
        (if (Variables|/Game/Purgatory/Paper_Pickup/BP_PaperPickUp.BP_PaperPickUp_C|GetbIsEndingPage _array_element)
          (CallFunction|PlayEndingCinematic))))))

(event Custom|SetCurrentPageVisibility
  (params (visibility :type ESlateVisibility%20Enum :default "Visible"))
  (bind _currentreadpage (Variables|UI|GetCurrentReadPage))
  ;[0.7653 1 0.6506] UI
  (Default|SetPageVisibility (Variables|UI|GetGameUI) visibility (Variables|/Game/Purgatory/Paper_Pickup/BP_PaperPickUp.BP_PaperPickUp_C|GetpageType (Variables|UI|GetCurrentReadPage)))
  (Default|SetClosePageVisibility (Variables|UI|GetGameUI) "Visible")
  (Default|SetPageText (Variables|UI|GetGameUI) (Variables|/Game/Purgatory/Paper_Pickup/BP_PaperPickUp.BP_PaperPickUp_C|GetContentText _currentreadpage) (Variables|/Game/Purgatory/Paper_Pickup/BP_PaperPickUp.BP_PaperPickUp_C|GetpageType _currentreadpage))
  (Variables|UI|SetbCanTurnPage true))

(event Custom|StartAmbience
  ;[1 1 1] Audio
  (if (not (Audio|Components|Audio|IsPlaying (Variables|Components|GetAmbienceSound)))
    (Audio|Components|Audio|Play (Variables|Components|GetAmbienceSound) 0.0)))

(event Custom|StopPlayingAmbience
  ;[1 1 1] Audio
  (Audio|Components|Audio|Stop (Variables|Components|GetAmbienceSound)))

(event Custom|ClearReadPage
  ;[1 0.9265 0.2541] Collision
  ;;[1 1 1] Activates Read Paper in UI
  ;;;[1 1 1] removes the read page promt after 4 sec
  (Default|SetReadPageVisibility (Variables|UI|GetGameUI) "Hidden"))

(event Custom|MoveToCheckpoint
  (params (CheckPointIndex :type Integer))
  (bind _debugmanager (Variables|Debug|GetDebugManager))
  (bind _levelstreamingmanager (Variables|Default|GetLevelStreamingManager))
  (bind _teleporttargets (Variables|/Game/Purgatory/DebugMode/BP_DebugManager.BP_DebugManager_C|GetTeleportTargets _debugmanager))
  (bind _output (Utilities|Array|Get(acopy) _teleporttargets CheckPointIndex))
  ;[1 0.7724 0] Debug Mode
  ;;[1 1 1] Moves player to checkpoint and restarts objects
  (if (< CheckPointIndex 7)
    (Utilities|IsValid (Variables|Debug|GetDebugManager)
      (:Is%20Valid
        (Utilities|IsValid _output
          (:Is%20Valid
            (Transformation|SetActorLocation (+ (Transformation|GetActorLocation _output) "0.000000, 0,100.000000") false true)
            ;;;[1 1 1] LevelStreaming
            (Utilities|IsValid _levelstreamingmanager
              (:Is%20Valid
                (Default|LoadLevel _levelstreamingmanager CheckPointIndex)))))))))

(event Custom|AddAllPapers
  (bind _debugmanager (Variables|Debug|GetDebugManager))
  (bind _paperpickups (Variables|/Game/Purgatory/DebugMode/BP_DebugManager.BP_DebugManager_C|GetPaperPickups _debugmanager))
  ;[1 0.7724 0] Debug Mode
  ;;[1 1 1] Add all pages to inventory
  (Utilities|IsValid (Variables|Debug|GetDebugManager)
    (:Is%20Valid
      (Variables|Papers|SetbHasPapers true)
      (if (> (Utilities|Array|Length _paperpickups) 0)
        (for _array_element _paperpickups
          (Utilities|Array|AddUnique (Variables|UI|GetReadablePages) _array_element))
        (Variables|UI|SetCurrentReadPage (Utilities|Array|Get(acopy) (Variables|UI|GetReadablePages)))))))

(event EventBeginPlay
  (bind _returnvalue (Game|GetPlayerController 0))
  (bind _playercameramanager (Variables|/Script/Engine.PlayerController|GetPlayerCameraManager _returnvalue))
  ;[1 0.4366 0.6192] Begin Play
  (CameraFades|StartCameraFade :self (Game|GetPlayerCameraManager 0) :FromAlpha 1.5 :Duration (Variables|Default|GetFadeInDuration))
  (bind _returnvalue_2 (Actor|GetActorOfClass "/Game/Purgatory/LevelStreaming/BP_LevelStreamingManager.BP_LevelStreamingManager_C"))
  (Variables|Default|SetLevelStreamingManager _returnvalue_2)
  ;;[1 1 1] Finds the debug Manager
  (bind _returnvalue_3 (Actor|GetActorOfClass "/Game/Purgatory/DebugMode/BP_DebugManager.BP_DebugManager_C"))
  (bind _output_get (Variables|Debug|SetDebugManager _returnvalue_3))
  (Utilities|IsValid _output_get
    (:Is%20Valid
      _)
    (:Is%20Not%20Valid
      (Development|PrintString "No DebugManager fonud in level!" true true "(R=1.000000,G=0.089264,B=0.000000,A=1.000000)")))
  (Audio|Components|Audio|Stop (Variables|Components|GetPushingBoxAudio))
  (bind _output_get_2 (Variables|Default|SetSFX (Utilities|Array|MakeArray (Variables|Default|GetWrongNote) (Variables|Default|GetCompletedWindup) (Variables|Default|GetResetWindup) (Variables|Components|GetPushingBoxAudio) (Variables|Components|GetFootStepAudio) (Variables|Default|GetLevelComplete))))
  (for _array_element _output_get_2
    (Audio|Components|Audio|Stop _array_element))
  (CallFunction|SetStart)
  (bind _outactors (Actor|GetAllActorswithInterface "/Game/Purgatory/Tests/Yunis/IRestart.IRestart_C"))
  (Variables|Restart|SetIRestartObjects _outactors)
  (bind _returnvalue_4 (UserInterface|CreateWidget "/Game/Purgatory/UI/BPW_GameUI.BPW_GameUI_C"))
  (bind _output_get_3 (Variables|UI|SetGameUI _returnvalue_4))
  (UserInterface|Viewport|AddtoViewport _output_get_3 0)
  (Input|SetInputModeGameOnly _returnvalue)
  (Variables|/Script/Engine.PlayerCameraManager|SetViewPitchMin _playercameramanager (Variables|Options|GetMinPitch))
  (Variables|/Script/Engine.PlayerCameraManager|SetViewPitchMax _playercameramanager (Variables|Options|GetMaxPitch)))

(event EventSetStart
  ;[1 0.5948 0.4333] IRestart
  (Variables|Restart|SetStartPosition (Transformation|GetActorLocation))
  (Variables|Restart|SetStartRotation (Transformation|GetActorRotation))
  (Utilities|Array|Clear (Variables|Papers|GetPapers)))

(event EventRestart
  (bind _currentcheckpoint (Variables|Checkpoints|GetCurrentCheckpoint))
  ;[1 0.5948 0.4333] IRestart
  ;;[1 1 1] RestartBook
  (Variables|Papers|SetCurrentPaper 0)
  (CallFunction|CloseBook)
  ;;[1 1 1] Blur Restart
  (Variables|Restart|SetbCanBlur false)
  (Restart|ResetBlur)
  (Utilities|Array|Clear (Variables|Papers|GetPapers))
  ;;[1 1 1] Restart
  (Transformation|SetActorLocation (Variables|Restart|GetStartPosition) false false)
  (Transformation|SetActorRotation (Variables|Restart|GetStartRotation))
  ;;[1 1 1] Reactivates the portal in the current checkpoint
  (Utilities|IsValid _currentcheckpoint
    (:Is%20Valid
      (Default|Activate (Variables|/Game/Purgatory/Checkpoint/BP_Checkpoint.BP_Checkpoint_C|GetEndPortal _currentcheckpoint)))))

(event EventTick
  (params (DeltaSeconds :type Float%20%28single-precision%29))
  (bind _charactermovement (Variables|Character|GetCharacterMovement))
  ;[1 0 0.05961] Tick
  ;;[1 1 1] Temprorary fix for grounded
  (Variables|Checks|SetbGrounded (AI|Components|NavMovement|IsMovingonGround _charactermovement))
  (if (Math|Vector|Equal(Vector) (Variables|/Script/Engine.MovementComponent|GetVelocity _charactermovement) "0, 0, 0" 0.0001)
    ;;[1 1 1] Long Idle Timer
    (if (not (Variables|Checks|GetbStartedLongIdleTimer))
      (Variables|Checks|SetbStartedLongIdleTimer true)
      (Utilities|Time|SetTimerbyFunctionName 0 "LongIdleTimer" (Variables|Checks|GetLongIdleTime) true))
    (elif (Variables|Checks|GetbStartedLongIdleTimer)
      (Variables|Checks|SetbStartedLongIdleTimer false)
      (Variables|Checks|SetbLongIdle false)
      (Utilities|Time|ClearTimerbyFunctionName 0 "LongIdleTimer"))))

(event Input|ActionEvents|InputActionTogglePause
  (params (Key :type Key%20Structure :default "None"))
  ;[0.7653 1 0.6506] UI
  (:Pressed
    (if (Game|IsGamePaused)
      (Default|ResumeGame (Variables|UI|GetPauseMenu))
      (else
        (CallFunction|CreatePauseMenu)))))

(event Input|KeyboardEvents|Q
  (params (Key :type Key%20Structure :default "None"))
  ;[0.4136 0.8797 1] Input
  ;;[1 1 1] Turn Page left with Q or MScroll Down
  (:Released
    (if (Variables|UI|GetbCanTurnPage)
      (CallFunction|TurnPage "NewEnumerator0"))))

(event Input|KeyboardEvents|R
  (params (Key :type Key%20Structure :default "None"))
  (bind _resetwindup (Variables|Default|GetResetWindup))
  ;[0.4136 0.8797 1] Input
  ;;[1 1 1] Hold R to restart
  (:Pressed
    (Restart|StartBlurTimer)
    (Audio|Components|Audio|Play _resetwindup 0.0))
  (:Released
    (Variables|Restart|SetbCanBlur true)
    (Utilities|Time|ClearTimerbyFunctionName 0 "BlurTimer")
    (Restart|ResetBlur)
    (Audio|Components|Audio|Stop _resetwindup)))

(event Input|KeyboardEvents|U
  (params (Key :type Key%20Structure :default "None"))
  ;[0.4136 0.8797 1] Input
  ;;[1 0.7724 0] Debug Mode
  ;;;[1 1 1] Add All pages
)

(event Input|KeyboardEvents|1
  (params (Key :type Key%20Structure :default "None"))
  ;[0.4136 0.8797 1] Input
  ;;[1 0.7724 0] Debug Mode
  ;;;[1 1 1] Moves to Different checkpoints
  (:Released
    (CallFunction|MovetoCheckpoint)))

(event Input|KeyboardEvents|2
  (params (Key :type Key%20Structure :default "None"))
  ;[0.4136 0.8797 1] Input
  ;;[1 0.7724 0] Debug Mode
  ;;;[1 1 1] Moves to Different checkpoints
  (:Released
    (CallFunction|MovetoCheckpoint 1)))

(event Input|KeyboardEvents|3
  (params (Key :type Key%20Structure :default "None"))
  ;[0.4136 0.8797 1] Input
  ;;[1 0.7724 0] Debug Mode
  ;;;[1 1 1] Moves to Different checkpoints
  (:Released
    (CallFunction|MovetoCheckpoint 2)))

(event Input|KeyboardEvents|4
  (params (Key :type Key%20Structure :default "None"))
  ;[0.4136 0.8797 1] Input
  ;;[1 0.7724 0] Debug Mode
  ;;;[1 1 1] Moves to Different checkpoints
  (:Released
    (CallFunction|MovetoCheckpoint 3)))

(event Input|MouseEvents|LeftMouseButton
  (params (Key :type Key%20Structure :default "None"))
  ;[0.4136 0.8797 1] Input
  ;;[1 1 1] Open Book with F or LMB
  (:Released
    (if (or (Utilities|IsValid (Variables|UI|GetCurrentReadPage)) (Variables|UI|GetbPaperIsVisible))
      (if (Variables|UI|GetbPaperIsVisible)
        (CallFunction|CloseBook)
        (else
          (CallFunction|OpenBook)))
      (Audio|PlaySoundatLocation "/Game/Purgatory/Sounds/SFX/SoundFiles/Open_notebook.Open_notebook" (Transformation|GetActorLocation) "0, 0, 0" 1.0 1.0 0.0 0 0 0))))

(event Input|KeyboardEvents|5
  (params (Key :type Key%20Structure :default "None"))
  ;[0.4136 0.8797 1] Input
  ;;[1 0.7724 0] Debug Mode
  ;;;[1 1 1] Moves to Different checkpoints
  (:Released
    (CallFunction|MovetoCheckpoint 4)))

(event Input|KeyboardEvents|6
  (params (Key :type Key%20Structure :default "None"))
  ;[0.4136 0.8797 1] Input
  ;;[1 0.7724 0] Debug Mode
  ;;;[1 1 1] Moves to Different checkpoints
  (:Released
    (CallFunction|MovetoCheckpoint 5)))

(event Input|KeyboardEvents|7
  (params (Key :type Key%20Structure :default "None"))
  ;[0.4136 0.8797 1] Input
  ;;[1 0.7724 0] Debug Mode
  ;;;[1 1 1] Moves to Different checkpoints
  (:Released
    (CallFunction|MovetoCheckpoint 6)))

(event Input|KeyboardEvents|8
  (params (Key :type Key%20Structure :default "None"))
  ;[0.4136 0.8797 1] Input
  ;;[1 0.7724 0] Debug Mode
  ;;;[1 1 1] Moves to Different checkpoints
)

(event Input|KeyboardEvents|G
  (params (Key :type Key%20Structure :default "None"))
  ;[0.4136 0.8797 1] Input
  ;;[1 0.7724 0] Debug Mode
  ;;;[1 1 1] Teleports object in room
  (:Released
    (CallFunction|Teleport)))

(event Input|KeyboardEvents|H
  (params (Key :type Key%20Structure :default "None"))
  ;[0.4136 0.8797 1] Input
  ;;[1 0.7724 0] Debug Mode
  ;;;[1 1 1] Deactivate current Portal Door
  (:Released
    (Default|Deactivate (Variables|/Game/Purgatory/Checkpoint/BP_Checkpoint.BP_Checkpoint_C|GetEndPortal (Variables|Checkpoints|GetCurrentCheckpoint)))))

(event Input|KeyboardEvents|F
  (params (Key :type Key%20Structure :default "None"))
  ;[0.4136 0.8797 1] Input
  ;;[1 1 1] Open Book with F or LMB
  (:Released
    (if (or (Utilities|IsValid (Variables|UI|GetCurrentReadPage)) (Variables|UI|GetbPaperIsVisible))
      (if (Variables|UI|GetbPaperIsVisible)
        (CallFunction|CloseBook)
        (else
          (CallFunction|OpenBook)))
      (Audio|PlaySoundatLocation "/Game/Purgatory/Sounds/SFX/SoundFiles/Open_notebook.Open_notebook" (Transformation|GetActorLocation) "0, 0, 0" 1.0 1.0 0.0 0 0 0))))

(event Input|KeyboardEvents|E
  (params (Key :type Key%20Structure :default "None"))
  ;[0.4136 0.8797 1] Input
  ;;[1 1 1] Turn Page right with e or MScroll Up
  (:Released
    (if (Variables|UI|GetbCanTurnPage)
      (CallFunction|TurnPage "NewEnumerator1"))))

(event Input|MouseEvents|MouseWheelDown
  (params (Key :type Key%20Structure :default "None"))
  ;[0.4136 0.8797 1] Input
  ;;[1 1 1] Turn Page left with Q or MScroll Down
  (:Released
    (if (Variables|UI|GetbCanTurnPage)
      (CallFunction|TurnPage "NewEnumerator0"))))

(event Input|MouseEvents|MouseWheelUp
  (params (Key :type Key%20Structure :default "None"))
  ;[0.4136 0.8797 1] Input
  ;;[1 1 1] Turn Page right with e or MScroll Up
  (:Released
    (if (Variables|UI|GetbCanTurnPage)
      (CallFunction|TurnPage "NewEnumerator1"))))

(fn ConstructionScript)

(fn RestartObjets
  (Variables|Papers|SetbHasPapers false)
  (for _array_element (Variables|Restart|GetIRestartObjects)
    (Class|IRestart|Restart(Message) _array_element)))

(fn BlurTimer
  (if (Variables|Restart|GetbCanBlur)
    (if (<= (Variables|Restart|GetCurrentScreenBlurOpacity) (Variables|Restart|GetRestartTime))
      (bind _output_get (Variables|Restart|SetCurrentScreenBlurOpacity (+ (Variables|Restart|GetCurrentScreenBlurOpacity) (Utilities|Time|GetWorldDeltaSeconds))))
      (Default|SetBGBlurOpacity (Variables|UI|GetGameUI) _output_get)
      (else
        (Restart|RestartObjets)))
    (else
      (Utilities|Time|ClearTimerbyFunctionName 0 "BlurTimer")
      (Audio|Components|Audio|Play (Variables|Default|GetCompletedWindup) 0.0))))

(fn ResetBlurTimer
  (if (>= (Variables|Restart|GetCurrentScreenBlurOpacity) 0.0)
    (bind _output_get (Variables|Restart|SetCurrentScreenBlurOpacity (- (Variables|Restart|GetCurrentScreenBlurOpacity) (* (Utilities|Time|GetWorldDeltaSeconds) 4.0))))
    (Default|SetBGBlurOpacity (Variables|UI|GetGameUI) _output_get)
    (else
      (Variables|Restart|SetbCanBlur true)
      (Utilities|Time|ClearTimerbyFunctionName 0 "ResetBlurTimer"))))

(fn ResetBlur
  (Utilities|Time|SetTimerbyFunctionName 0 "ResetBlurTimer" (Utilities|Time|GetWorldDeltaSeconds) true))

(fn CreatePauseMenu
  (bind _returnvalue (Game|GetPlayerController 0))
  (Utilities|IsValid (Variables|UI|GetPauseMenu)
    (:Is%20Valid
      _)
    (:Is%20Not%20Valid
      (bind _returnvalue_2 (UserInterface|CreateWidget "/Game/Purgatory/UI/BPW_PauseMenu.BPW_PauseMenu_C"))
      (bind _output_get (Variables|UI|SetPauseMenu _returnvalue_2))))
  (UserInterface|Viewport|AddtoViewport _output_get 0)
  (Variables|/Script/Engine.PlayerController|SetbShowMouseCursor _returnvalue true)
  (Input|SetInputModeGameandUI _returnvalue (Variables|UI|GetPauseMenu) "DoNotLock" false)
  (Widget|SetVisibility (Variables|/Game/Purgatory/UI/BPW_PauseMenu.BPW_PauseMenu_C|GetPauseMenu (Variables|UI|GetPauseMenu)) "Visible")
  (Game|SetGamePaused true))

(fn LongIdleTimer
  (Variables|Checks|SetbLongIdle true))

(fn StartBlurTimer
  (Utilities|Time|SetTimerbyFunctionName 0 "BlurTimer" (Utilities|Time|GetWorldDeltaSeconds) true))