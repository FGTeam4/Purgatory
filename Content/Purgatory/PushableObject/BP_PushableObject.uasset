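; Pushable object in Purgatory that can ride on looping boxes and reset to its start transform through restart events.
; Box overlap links it with the looping box and stores their height offset, which TeleportWithLoopable uses to reposition it.
; A looping timer unlinks them once overlap ends.
; While Lars overlaps the collider, a timed one-sided line trace plays wall-hit audio on non-Lars hits.
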(event OnComponentBeginOverlap(Box)
  (params (OverlappedComponent :type Primitive%20Component%20Object%20Reference) (OtherActor :type Actor%20Object%20Reference) (OtherComp :type Primitive%20Component%20Object%20Reference) (OtherBodyIndex :type Integer) (bFromSweep :type Boolean) (SweepResult :type Hit%20Result%20Structure%20%28by%20ref%29))
  ;[1 1 1] to see if the pushableObject has a loopingBox under it. if so, set that object as currentLoopingBox
  (bind _asbp_looping_box (Utilities|Casting|CastToBP_LoopingBox OtherActor))
  (if (not (== _asbp_looping_box (Variables|Default|GetCurrentLoopingBox)))
    (bind _output_get (Variables|Default|SetCurrentLoopingBox _asbp_looping_box))
    (Variables|/Game/Purgatory/Tests/Alex/BP_LoopingBox.BP_LoopingBox_C|SetCurrentPushableObject _output_get self)
    (Variables|Default|SetHeightDifferenceOnLoopBox (Math|Float|Absolute(Float) (- (.z (Transformation|GetActorLocation)) (.z (Transformation|GetActorLocation (Variables|Default|GetCurrentLoopingBox))))))))

(event OnComponentBeginOverlap(Collider)
  (params (OverlappedComponent :type Primitive%20Component%20Object%20Reference) (OtherActor :type Actor%20Object%20Reference) (OtherComp :type Primitive%20Component%20Object%20Reference) (OtherBodyIndex :type Integer) (bFromSweep :type Boolean) (SweepResult :type Hit%20Result%20Structure%20%28by%20ref%29))
  ;[1 1 1] If box hits wall whne pushing, play sound
  (Utilities|Casting|CastToBP_Character_Lars OtherActor)
  (bind _returnvalue (Utilities|Time|SetTimerbyEvent (delegate Custom|CheckForObjects) 0.1 true))
  (Variables|Default|SetCheckTimerHandle _returnvalue))

(event OnComponentEndOverlap(Collider)
  (params (OverlappedComponent :type Primitive%20Component%20Object%20Reference) (OtherActor :type Actor%20Object%20Reference) (OtherComp :type Primitive%20Component%20Object%20Reference) (OtherBodyIndex :type Integer))
  ;[1 1 1] Stop Timer Handle
  (Utilities|Time|PauseTimerbyHandle (Variables|Default|GetCheckTimerHandle)))

(event Custom|IsStillOverlaping
  ;[1 1 1] Check to see if the pushable object is still colliding with the loopable object
  (if (not (Collision|IsOverlappingActor (Variables|Default|GetBox) (Variables|Default|GetCurrentLoopingBox) :!class /Script/Engine.PrimitiveComponent))
    (Utilities|IsValid (Variables|Default|GetCurrentLoopingBox)
      (:Is%20Valid
        (Variables|/Game/Purgatory/Tests/Alex/BP_LoopingBox.BP_LoopingBox_C|SetCurrentPushableObject (Variables|Default|GetCurrentLoopingBox) 0)
        (Variables|Default|SetCurrentLoopingBox 0)))))

(event Custom|TeleportWithLoopable
  (bind _currentloopingbox (Variables|Default|GetCurrentLoopingBox))
  (bind _returnvalue (Transformation|GetActorLocation _currentloopingbox))
  ;[1 1 1] Teleport with touch looping box
  (Utilities|IsValid (Variables|Default|GetCurrentLoopingBox)
    (:Is%20Valid
      (Transformation|SetActorLocation (Math|Vector|MakeVector (.x _returnvalue) (.y _returnvalue) (+ (.z _returnvalue) (Variables|Default|GetHeightDifferenceOnLoopBox))) false false))))

(event Custom|CheckForObjects
  (bind _returnvalue (Transformation|GetActorLocation))
  (bind _checkdistance (Variables|Default|GetCheckDistance))
  (bind (_x _y _z) (Math|Vector|BreakVector _returnvalue))
  (bind _returnvalue_2 (+ _z _checkdistance))
  (bind _returnvalue_3 (Math|Vector|MakeVector _x _y _returnvalue_2))
  ;[1 1 1] If box hits wall whne pushing, play sound
  (bind (_outhit _returnvalue_4) (Collision|LineTraceByChannel _returnvalue_3 (+ _returnvalue_3 (* (Transformation|GetActorRightVector) (* _checkdistance -1.0))) "TraceTypeQuery1" false 0 "None"))
  (if _returnvalue_4
    (Utilities|Casting|CastToBP_Character_Lars (.HitActor (Collision|BreakHitResult _outhit))
      (:CastFailed
        (if (not (Audio|Components|Audio|IsPlaying (Variables|Default|GetHitWallAudio)))
          (Audio|Components|Audio|Play (Variables|Default|GetHitWallAudio) 0.0))))))

(event EventBeginPlay
  (Audio|Components|Audio|Stop (Variables|Default|GetHitWallAudio))
  ;[1 1 1] Initialize variables
  (CallFunction|SetStart)
  (bind _asbp_character_lars (Utilities|Casting|CastToBP_Character_Lars (Game|GetPlayerCharacter 0))
    (:then
      (Variables|Default|SetCharacter _asbp_character_lars))
    (:CastFailed
      _))
  ;[1 1 1] Check to see if the pushable object is still colliding with the loopable object
  (Utilities|Time|SetTimerbyEvent (delegate Custom|IsStillOverlaping) 0.5 true))

(event EventSetStart
  ;[1 1 1] IRestart
  (Variables|Default|SetStartTransform (Transformation|GetActorTransform)))

(event EventRestart
  ;[1 1 1] IRestart
  (Transformation|SetActorTransform (Variables|Default|GetStartTransform))
  (Variables|Default|SetCurrentLoopingBox 0))

(fn ConstructionScript)