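; Test trigger actor that moves a referenced Box through up to five preset transforms, one step each time the player leaves its trigger.
; A loop counter selects the transform and wraps to zero past MaxLoops.
; A successful move reporting a nonzero sweep impact flags the box as stuck, so the next end overlap by any actor returns it to StartPoint.
; Restart clears counter and flag; construction applies the chosen mesh to the box.
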(event OnComponentEndOverlap(Trigger)
  (params (OverlappedComponent :type Primitive%20Component%20Object%20Reference) (OtherActor :type Actor%20Object%20Reference) (OtherComp :type Primitive%20Component%20Object%20Reference) (OtherBodyIndex :type Integer))
  (if (Variables|Default|GetStuck)
    (Variables|Default|SetStuck false)
    (Transformation|SetActorTransform (Variables|Default|GetBox) (Variables|Default|GetStartPoint) false true)
    (elif (== OtherActor (Game|GetPlayerCharacter 0))
      (bind _output_get (Variables|Default|SetLoop (+ (Variables|Default|GetLoop) 1)))
      (if (> _output_get (Variables|Default|GetMaxLoops))
        (bind _output_get_2 (Variables|Default|SetLoop 0)))
      (switch int _output_get_2
        (:0
          (Variables|Default|SetNewTransform (Variables|Default|GetTransform0)))
        (:1
          (Variables|Default|SetNewTransform (Variables|Default|GetTransform1)))
        (:2
          (Variables|Default|SetNewTransform (Variables|Default|GetTransform2)))
        (:3
          (Variables|Default|SetNewTransform (Variables|Default|GetTransform3)))
        (:4
          (Variables|Default|SetNewTransform (Variables|Default|GetTransform4))))
      (bind (_sweephitresult _returnvalue) (Transformation|SetActorTransform (Variables|Default|GetBox) (Variables|Default|GetNewTransform) (Variables|Default|GetSweep) (Variables|Default|GetTeleport)))
      (if _returnvalue
        (if (Math|Vector|NotEqual(Vector) (.ImpactPoint (Collision|BreakHitResult _sweephitresult)) "0, 0, 0" 0.0)
          (Variables|Default|SetStuck true))))))

(event EventRestart
  (Variables|Default|SetLoop 0)
  (Variables|Default|SetStuck false))

(event EventBeginPlay
  (Transformation|SetActorTransform (Variables|Default|GetBox) (Variables|Default|GetTransform0) false true))

(fn ConstructionScript
  (Components|StaticMesh|SetStaticMesh (Variables|/Game/Purgatory/Tests/Alex/BP_LoopingBox.BP_LoopingBox_C|GetStaticMesh (Variables|Default|GetBox)) (Variables|Default|GetMesh)))