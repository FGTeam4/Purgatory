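; Pushable box test actor that slides in one of four fixed directions while the player character touches it.
; Four side collision volumes set a contact flag and direction index on overlap, with numbering that does not match their compass names.
; Tick applies that direction's offset with a sweep, unscaled by delta time.
; Restart returns it to its BeginPlay transform; the construction script applies its mesh and material.
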(event OnComponentEndOverlap(WestCollision)
  (params (OverlappedComponent :type Primitive%20Component%20Object%20Reference) (OtherActor :type Actor%20Object%20Reference) (OtherComp :type Primitive%20Component%20Object%20Reference) (OtherBodyIndex :type Integer))
  ;[1 1 1] nummer etc. är huller om buller just nu, behöver städas upp före CPP
  (if (== OtherActor (Game|GetPlayerCharacter 0))
    (Variables|Default|SetContact false)))

(event OnComponentBeginOverlap(EastCollision)
  (params (OverlappedComponent :type Primitive%20Component%20Object%20Reference) (OtherActor :type Actor%20Object%20Reference) (OtherComp :type Primitive%20Component%20Object%20Reference) (OtherBodyIndex :type Integer) (bFromSweep :type Boolean) (SweepResult :type Hit%20Result%20Structure%20%28by%20ref%29))
  ;[1 1 1] nummer etc. är huller om buller just nu, behöver städas upp före CPP
  (if (== OtherActor (Game|GetPlayerCharacter 0))
    (Variables|Default|SetContact true)
    (Variables|Default|SetDirection 0)))

(event OnComponentEndOverlap(EastCollision)
  (params (OverlappedComponent :type Primitive%20Component%20Object%20Reference) (OtherActor :type Actor%20Object%20Reference) (OtherComp :type Primitive%20Component%20Object%20Reference) (OtherBodyIndex :type Integer))
  ;[1 1 1] nummer etc. är huller om buller just nu, behöver städas upp före CPP
  (if (== OtherActor (Game|GetPlayerCharacter 0))
    (Variables|Default|SetContact false)))

(event OnComponentBeginOverlap(NorthCollision)
  (params (OverlappedComponent :type Primitive%20Component%20Object%20Reference) (OtherActor :type Actor%20Object%20Reference) (OtherComp :type Primitive%20Component%20Object%20Reference) (OtherBodyIndex :type Integer) (bFromSweep :type Boolean) (SweepResult :type Hit%20Result%20Structure%20%28by%20ref%29))
  ;[1 1 1] nummer etc. är huller om buller just nu, behöver städas upp före CPP
  (if (== OtherActor (Game|GetPlayerCharacter 0))
    (Variables|Default|SetContact true)
    (Variables|Default|SetDirection 3)))

(event OnComponentEndOverlap(NorthCollision)
  (params (OverlappedComponent :type Primitive%20Component%20Object%20Reference) (OtherActor :type Actor%20Object%20Reference) (OtherComp :type Primitive%20Component%20Object%20Reference) (OtherBodyIndex :type Integer))
  ;[1 1 1] nummer etc. är huller om buller just nu, behöver städas upp före CPP
  (if (== OtherActor (Game|GetPlayerCharacter 0))
    (Variables|Default|SetContact false)))

(event OnComponentBeginOverlap(SouthCollision)
  (params (OverlappedComponent :type Primitive%20Component%20Object%20Reference) (OtherActor :type Actor%20Object%20Reference) (OtherComp :type Primitive%20Component%20Object%20Reference) (OtherBodyIndex :type Integer) (bFromSweep :type Boolean) (SweepResult :type Hit%20Result%20Structure%20%28by%20ref%29))
  ;[1 1 1] nummer etc. är huller om buller just nu, behöver städas upp före CPP
  (if (== OtherActor (Game|GetPlayerCharacter 0))
    (Variables|Default|SetContact true)
    (Variables|Default|SetDirection 1)))

(event OnComponentBeginOverlap(WestCollision)
  (params (OverlappedComponent :type Primitive%20Component%20Object%20Reference) (OtherActor :type Actor%20Object%20Reference) (OtherComp :type Primitive%20Component%20Object%20Reference) (OtherBodyIndex :type Integer) (bFromSweep :type Boolean) (SweepResult :type Hit%20Result%20Structure%20%28by%20ref%29))
  ;[1 1 1] nummer etc. är huller om buller just nu, behöver städas upp före CPP
  (if (== OtherActor (Game|GetPlayerCharacter 0))
    (Variables|Default|SetContact true)
    (Variables|Default|SetDirection 2)))

(event OnComponentEndOverlap(SouthCollision)
  (params (OverlappedComponent :type Primitive%20Component%20Object%20Reference) (OtherActor :type Actor%20Object%20Reference) (OtherComp :type Primitive%20Component%20Object%20Reference) (OtherBodyIndex :type Integer))
  ;[1 1 1] nummer etc. är huller om buller just nu, behöver städas upp före CPP
  (if (== OtherActor (Game|GetPlayerCharacter 0))
    (Variables|Default|SetContact false)))

(event EventRestart
  (Variables|Default|SetContact false)
  (Transformation|SetActorTransform (Variables|Default|GetStartTransform)))

(event EventBeginPlay
  (Variables|Default|SetStartTransform (Transformation|GetActorTransform)))

(event EventTick
  (params (DeltaSeconds :type Float%20%28single-precision%29))
  ;[1 1 1] nummer etc. är huller om buller just nu, behöver städas upp före CPP
  (if (Variables|Default|GetContact)
    (switch int (Variables|Default|GetDirection)
      (:0
        (Variables|Default|Setmovement (Variables|Default|GetMoveNorth)))
      (:1
        (Variables|Default|Setmovement (Variables|Default|GetMoveEast)))
      (:2
        (Variables|Default|Setmovement (Variables|Default|GetMoveSouth)))
      (:3
        (Variables|Default|Setmovement (Variables|Default|GetMoveWest))))
    (Transformation|AddActorWorldOffset (Variables|Default|Getmovement) true)))

(fn ConstructionScript
  (Components|StaticMesh|SetStaticMesh (Variables|Default|GetStaticMesh) (Variables|Default|GetMesh))
  (Rendering|Material|SetMaterial (Variables|Default|GetStaticMesh) 0 (Variables|Default|GetMaterial)))