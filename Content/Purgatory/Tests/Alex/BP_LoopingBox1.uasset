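; BP_LoopingBox1 is a test actor with a configurable mesh that steps through preset transforms whenever its Lars OnTeleport event fires.
; BeginPlay records the placed transform, then snaps to the first preset; each event advances Loop, wrapping past MaxLoops.
; A successful move with a nonzero sweep impact point sets Stuck, so the next event returns the box to its start.
; Restart restores that start and clears both states.
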(event OnTeleport(Lars)
  (Development|PrintString "Hello")
  (if (Variables|Default|GetStuck)
    (Variables|Default|SetStuck false)
    (Transformation|SetActorTransform (Variables|Default|GetstartTransform) false true)
    (else
      (bind _output_get (Variables|Default|SetLoop (+ (Variables|Default|GetLoop) 1)))
      (if (> _output_get (Variables|Default|GetMaxLoops))
        (Variables|Default|SetLoop 0))
      (bind (_sweephitresult _returnvalue) (Transformation|SetActorTransform (Utilities|Array|Get(acopy) (Variables|Default|GetTransforms) (Variables|Default|GetLoop)) (Variables|Default|GetSweep) (Variables|Default|GetTeleport)))
      (Development|PrintString "Hello")
      (if _returnvalue
        (if (Math|Vector|NotEqual(Vector) (.ImpactPoint (Collision|BreakHitResult _sweephitresult)) "0, 0, 0" 0.0)
          (Variables|Default|SetStuck true))))))

(event EventBeginPlay
  (CallFunction|SetStart)
  (Transformation|SetActorTransform (Utilities|Array|Get(acopy) (Variables|Default|GetTransforms)) false true))

(event EventRestart
  (Transformation|SetActorTransform (Variables|Default|GetstartTransform))
  (Variables|Default|SetLoop 0)
  (Variables|Default|SetStuck false))

(event EventSetStart
  (Variables|Default|SetstartTransform (Transformation|GetActorTransform)))

(fn ConstructionScript
  (Components|StaticMesh|SetStaticMesh (Variables|Default|GetStaticMesh) (Variables|Default|GetMesh)))