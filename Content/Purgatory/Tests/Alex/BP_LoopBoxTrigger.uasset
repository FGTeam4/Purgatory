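; Test trigger that steps a linked Box actor's transform by PerLoopChange each time the player leaves it, counting loops.
; Past MaxLoops it zeroes Loop before applying BackToStart, whose Loop-scaled subtraction therefore appears to yield no offset.
; Moves are swept, and an impact sets Stuck, so the next end overlap by any actor teleports Box to its BeginPlay transform.
; The construction script applies Mesh to Box.
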(event OnComponentEndOverlap(Trigger)
  (params (OverlappedComponent :type Primitive%20Component%20Object%20Reference) (OtherActor :type Actor%20Object%20Reference) (OtherComp :type Primitive%20Component%20Object%20Reference) (OtherBodyIndex :type Integer))
  (bind (_returnvalue _returnvalue2 _returnvalue3 _returnvalue4 _returnvalue5) (Utilities|BacktoStart))
  (bind (_returnvalue_2 _returnvalue2_2 _returnvalue3_2 _returnvalue4_2 _returnvalue5_2) (Utilities|TransformChangePerLoop))
  (if (Variables|Default|GetStuck)
    (Variables|Default|SetStuck false)
    (Transformation|SetActorTransform (Variables|Default|GetBox) (Variables|Default|GetStartPoint) false true)
    (elif (== OtherActor (Game|GetPlayerCharacter 0))
      (bind _output_get (Variables|Default|SetLoop (+ (Variables|Default|GetLoop) 1)))
      (if (> _output_get (Variables|Default|GetMaxLoops))
        (Variables|Default|SetLoop 0)
        (bind (_sweephitresult _returnvalue_3) (Transformation|SetActorTransform (Variables|Default|GetBox) (Math|Transform|MakeTransform _returnvalue (Math|Rotator|MakeRotator _returnvalue2 _returnvalue3 _returnvalue4) _returnvalue5) true true))
        (if _returnvalue_3
          (if (Math|Vector|NotEqual(Vector) (.ImpactPoint (Collision|BreakHitResult _sweephitresult)) "0,0.000000, 0" 0.0)
            (Variables|Default|SetStuck true :!label _label)))
        (else
          (bind (_sweephitresult_2 _returnvalue_4) (Transformation|SetActorTransform (Variables|Default|GetBox) (Math|Transform|MakeTransform _returnvalue_2 (Math|Rotator|MakeRotator _returnvalue2_2 _returnvalue3_2 _returnvalue4_2) _returnvalue5_2) true true))
          (if _returnvalue_4
            (if (Math|Vector|NotEqual(Vector) (.ImpactPoint (Collision|BreakHitResult _sweephitresult_2)) "0, 0, 0" 0.0)
              (goto _label))))))))

(event EventBeginPlay
  (Variables|Default|SetStartPoint (Transformation|GetActorTransform (Variables|Default|GetBox))))

(fn ConstructionScript
  (Components|StaticMesh|SetStaticMesh (Variables|/Game/Purgatory/Tests/Alex/BP_LoopingBox.BP_LoopingBox_C|GetStaticMesh (Variables|Default|GetBox)) (Variables|Default|GetMesh)))