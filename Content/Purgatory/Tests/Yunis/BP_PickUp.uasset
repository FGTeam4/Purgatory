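; BP_PickUp is a test actor for a physics object that can be picked up, dropped and reset.
; BeginPlay caches the mesh's collision profile and the actor's starting location.
; OnPickUp disables physics and collision, leaving attachment to be done elsewhere, while Drop restores both and detaches the mesh.
; Reset moves the actor to its start and, if held, reuses Drop's release steps without clearing PickedUp.
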(event Custom|OnPickUp
  (if (Variables|Default|GetbPickedUp)
    _
    (else
      _))
  (Variables|Default|SetbPickedUp true)
  (Physics|SetSimulatePhysics (Variables|Default|GetStaticMesh) false)
  (Collision|SetCollisionProfileName (Variables|Default|GetStaticMesh) "NoCollision" true :!class /Script/Engine.PrimitiveComponent))

(event Custom|Drop
  (if (Variables|Default|GetbPickedUp)
    (Variables|Default|SetbPickedUp false)
    (Collision|SetCollisionProfileName (Variables|Default|GetStaticMesh) (Variables|Default|GetOriginalCollisionProfile) true :!class /Script/Engine.PrimitiveComponent)
    (Physics|SetSimulatePhysics (Variables|Default|GetStaticMesh) true)
    (Transformation|DetachFromComponent (Variables|Default|GetStaticMesh) "KeepWorld" "KeepWorld" "KeepWorld" true)))

(event Custom|Reset
  (Transformation|SetActorLocation (Variables|Default|GetOriginalPosition) false false)
  (if (Variables|Default|GetbPickedUp)
    (Collision|SetCollisionProfileName (Variables|Default|GetStaticMesh) (Variables|Default|GetOriginalCollisionProfile) true :!class /Script/Engine.PrimitiveComponent)
    (Physics|SetSimulatePhysics (Variables|Default|GetStaticMesh) true)
    (Transformation|DetachFromComponent (Variables|Default|GetStaticMesh) "KeepWorld" "KeepWorld" "KeepWorld" true)))

(event EventBeginPlay
  (Variables|Default|SetOriginalCollisionProfile (Collision|GetCollisionProfileName (Variables|Default|GetStaticMesh)))
  (Utilities|Casting|CastToBP_Character_Lars (Game|GetPlayerCharacter 0))
  (Variables|Default|SetHoldingTarget 0)
  (Variables|Default|SetOriginalPosition (Transformation|GetActorLocation)))

(event Collision|EventActorBeginOverlap
  (params (OtherActor :type Actor%20Object%20Reference)))

(event EventTick
  (params (DeltaSeconds :type Float%20%28single-precision%29)))

(fn ConstructionScript)