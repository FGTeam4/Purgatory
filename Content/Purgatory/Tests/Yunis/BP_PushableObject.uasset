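; BP_PushableObject is a pushable object that follows the BP_LoopingBox it touches when the Lars character teleports.
; Box overlap stores the looping box and the absolute height offset from it, while a looping timer clears the reference once overlap ends.
; The character's teleport event snaps the object to that box's X/Y at the stored height above it.
; Restart restores the transform saved at BeginPlay and forgets the box.
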(event OnComponentBeginOverlap(Box)
  (params (OverlappedComponent :type Primitive%20Component%20Object%20Reference) (OtherActor :type Actor%20Object%20Reference) (OtherComp :type Primitive%20Component%20Object%20Reference) (OtherBodyIndex :type Integer) (bFromSweep :type Boolean) (SweepResult :type Hit%20Result%20Structure%20%28by%20ref%29))
  (bind _asbp_looping_box (Utilities|Casting|CastToBP_LoopingBox OtherActor))
  (if (not (== _asbp_looping_box (Variables|Default|GetCurrentLoopingBox)))
    (Variables|Default|SetCurrentLoopingBox _asbp_looping_box)
    (Variables|Default|SetHeightDifferenceOnLoopBox (Math|Float|Absolute(Float) (- (.z (Transformation|GetActorLocation)) (.z (Transformation|GetActorLocation (Variables|Default|GetCurrentLoopingBox))))))))

(event Custom|IsStillOverlaping
  ;[1 1 1] Check to see if the pushable object is still colliding with the loopable object
  (if (not (Collision|IsOverlappingActor (Variables|Default|GetBox) (Variables|Default|GetCurrentLoopingBox) :!class /Script/Engine.PrimitiveComponent))
    (Variables|Default|SetCurrentLoopingBox 0)))

(event Custom|TeleportWithBox
  (bind _currentloopingbox (Variables|Default|GetCurrentLoopingBox))
  (bind _returnvalue (Transformation|GetActorLocation _currentloopingbox))
  ;[1 1 1] Teleport with touch looping box
  (Utilities|IsValid (Variables|Default|GetCurrentLoopingBox)
    (:Is%20Valid
      (Transformation|SetActorLocation (Math|Vector|MakeVector (.x _returnvalue) (.y _returnvalue) (+ (.z _returnvalue) (Variables|Default|GetHeightDifferenceOnLoopBox))) false false))))

(event EventBeginPlay
  (CallFunction|SetStart)
  (bind _asbp_character_lars (Utilities|Casting|CastToBP_Character_Lars (Game|GetPlayerCharacter 0))
    (:then
      (bind _output_get (Variables|Default|SetCharacter _asbp_character_lars))
      (EventDispatchers|BindEventtoOnTeleport _output_get (delegate Custom|TeleportWithBox)))
    (:CastFailed
      _))
  ;[1 1 1] Check to see if the pushable object is still colliding with the loopable object
  (Utilities|Time|SetTimerbyEvent (delegate Custom|IsStillOverlaping) 0.5 true))

(event Collision|EventActorBeginOverlap
  (params (OtherActor :type Actor%20Object%20Reference)))

(event EventTick
  (params (DeltaSeconds :type Float%20%28single-precision%29)))

(event EventSetStart
  (Variables|Default|SetStartTransform (Transformation|GetActorTransform)))

(event EventRestart
  (Transformation|SetActorTransform (Variables|Default|GetStartTransform))
  (Variables|Default|SetCurrentLoopingBox 0))

(fn ConstructionScript)