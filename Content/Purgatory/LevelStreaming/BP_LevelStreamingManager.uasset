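; Level streaming manager that switches the active level among a set of streaming volumes by index.
; LoadLevel ignores a request for the current volume; otherwise it records the old one as LastLevel and makes the requested one current.
; It then calls LoadThisLevel and StreamLevels on the new volume before calling UnloadThisLevel on the previous one, leaving the streaming work to the volumes themselves.
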(event Custom|LoadLevel
  (params (Index :type Integer))
  (bind _streamingvolumes (Variables|Default|GetStreamingVolumes))
  (bind _output (Utilities|Array|Get(acopy) _streamingvolumes Index))
  (if (!= _output (Variables|Default|GetCurrentLevel))
    (Variables|Default|SetLastLevel (Variables|Default|GetCurrentLevel))
    (bind _output_get (Variables|Default|SetCurrentLevel _output))
    (Default|LoadThisLevel _output_get)
    (Default|StreamLevels (Variables|Default|GetCurrentLevel))
    (Default|UnloadThisLevel (Variables|Default|GetLastLevel))))

(event EventBeginPlay)

(event Collision|EventActorBeginOverlap
  (params (OtherActor :type Actor%20Object%20Reference)))

(event EventTick
  (params (DeltaSeconds :type Float%20%28single-precision%29)))

(fn ConstructionScript)