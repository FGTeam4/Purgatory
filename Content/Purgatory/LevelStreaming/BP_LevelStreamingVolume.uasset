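; Trigger volume that streams levels in and out when the Lars player character enters its box.
; The overlap loads LevelsToLoad without blocking, adds every IRestart actor to the character's IRestartObjects list, then unloads LevelToUnload.
; Separate LoadThisLevel and UnloadThisLevel events load or unload a single Level on demand, with loading also registering IRestart actors.
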(event OnComponentBeginOverlap(Box)
  (params (OverlappedComponent :type Primitive%20Component%20Object%20Reference) (OtherActor :type Actor%20Object%20Reference) (OtherComp :type Primitive%20Component%20Object%20Reference) (OtherBodyIndex :type Integer) (bFromSweep :type Boolean) (SweepResult :type Hit%20Result%20Structure%20%28by%20ref%29))
  (if (== OtherActor (Variables|Default|GetCharacter))
    (CallFunction|StreamLevels)))

(event Custom|StreamLevels
  (bind _levelstoload (Variables|LevelStreaming|GetLevelsToLoad))
  (bind _leveltounload (Variables|LevelStreaming|GetLevelToUnload))
  (if (Utilities|Name|NotEqual(Name) _levelstoload "None")
    (Game|LoadStreamLevel(byName) _levelstoload true))
  (bind _outactors (Actor|GetAllActorswithInterface "/Game/Purgatory/Tests/Yunis/IRestart.IRestart_C"))
  (for _array_element _outactors
    (Utilities|Array|AddUnique (Variables|/Game/Purgatory/Character/Lars/BP_Character_Lars.BP_Character_Lars_C|GetIRestartObjects (Variables|Default|GetCharacter)) _array_element))
  (if (Utilities|Name|NotEqual(Name) _leveltounload "None")
    (Game|UnloadStreamLevel(byName) _leveltounload false)))

(event Custom|LoadThisLevel
  (bind _level (Variables|LevelStreaming|GetLevel))
  (if (Utilities|Name|NotEqual(Name) _level "None")
    (Game|LoadStreamLevel(byName) _level true)
    (bind _outactors (Actor|GetAllActorswithInterface "/Game/Purgatory/Tests/Yunis/IRestart.IRestart_C"))
    (for _array_element _outactors
      (Utilities|Array|AddUnique (Variables|/Game/Purgatory/Character/Lars/BP_Character_Lars.BP_Character_Lars_C|GetIRestartObjects (Variables|Default|GetCharacter)) _array_element))))

(event Custom|UnloadThisLevel
  (bind _level (Variables|LevelStreaming|GetLevel))
  (if (Utilities|Name|NotEqual(Name) _level "None")
    (Game|UnloadStreamLevel(byName) _level false)))

(event EventBeginPlay
  (bind _asbp_character_lars (Utilities|Casting|CastToBP_Character_Lars (Game|GetPlayerCharacter 0)))
  (Variables|Default|SetCharacter _asbp_character_lars))

(event Collision|EventActorBeginOverlap
  (params (OtherActor :type Actor%20Object%20Reference)))

(event EventTick
  (params (DeltaSeconds :type Float%20%28single-precision%29)))

(fn ConstructionScript)